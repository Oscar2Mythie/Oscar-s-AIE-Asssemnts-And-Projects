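; Gold door button actor that the player presses once to open its linked button-locked door.
; A sphere overlap toggles a "press to interact" widget while the button is unpressed.
; It binds to the player's world interaction event, checks a distance limit, then eases the button spring down and opens the door.
; The first opening increments and prints the DoorsOpen count on the GM_Gamplay actor found at BeginPlay.
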(event OnComponentBeginOverlap(Sphere)
  (params (OverlappedComponent :type Primitive%20Component%20Object%20Reference) (OtherActor :type Actor%20Object%20Reference) (OtherComp :type Primitive%20Component%20Object%20Reference) (OtherBodyIndex :type Integer) (bFromSweep :type Boolean) (SweepResult :type Hit%20Result%20Structure%20%28by%20ref%29))
  (if (not (Variables|Default|GetIs_Pressed))
    (Rendering|SetVisibility (Variables|Default|GetWidget) true false)))

(event OnComponentEndOverlap(Sphere)
  (params (OverlappedComponent :type Primitive%20Component%20Object%20Reference) (OtherActor :type Actor%20Object%20Reference) (OtherComp :type Primitive%20Component%20Object%20Reference) (OtherBodyIndex :type Integer))
  (Rendering|SetVisibility (Variables|Default|GetWidget) false false))

(event Custom|Player_interact_Button
  (bind _gm_gameplay (Variables|Default|GetGM_Gameplay))
  (if (<= (Math|Vector|Distance(Vector) (Transformation|GetActorLocation self) (Transformation|GetActorLocation (Variables|Default|GetPlayer))) 2e+02)
    (if (not (Variables|Default|GetIs_Pressed))
      (Variables|Default|SetIs_Pressed true)
      (Components|MoveComponentTo (Variables|Default|GetButton_Spring) "0.000000,0.000000,-26.000000" "0, 0, 0" true true 0.5 false)
      (Utilities|FlowControl|Sequence
        (:then_0
          (Default|OpenButtonLockedDoor (Variables|Default|GetButton_Locked_Door))
          (Rendering|SetVisibility (Variables|Default|GetWidget) false false))
        (:then_1
          (if (Variables|Default|Getfirst%20time%20opened)
            (bind _output_get (Variables|/Game/Game_Modes/GM_Gamplay.GM_Gamplay_C|SetDoors_Open _gm_gameplay (+ (Variables|/Game/Game_Modes/GM_Gamplay.GM_Gamplay_C|GetDoors_Open _gm_gameplay) 1)))
            (Variables|Default|Setfirst%20time%20opened false)
            (Development|PrintString (Utilities|String|ToString(Integer) _output_get))))))))

(event EventBeginPlay
  (Utilities|FlowControl|Sequence
    (:then_0
      (bind _aswd_hud_press_to_interact_icon (Utilities|Casting|CastToWD_HUD_Press_to_interact_icon (UserInterface|GetUserWidgetObject (Variables|Default|GetWidget))))
      (Variables|Default|SetAs%20WD%20HUD%20Press%20to%20Interact%20Icon _aswd_hud_press_to_interact_icon)
      (bind _outactors (Actor|GetAllActorsOfClass "/Game/Game_Modes/GM_Gamplay.GM_Gamplay_C"))
      (Variables|Default|SetGM_Gameplay (Utilities|Array|Get(acopy) _outactors)))
    (:then_1
      (Rendering|SetVisibility (Variables|Default|GetWidget) false false))
    (:then_2
      (EventDispatchers|BindEventtoWorldInteraction (Variables|Default|GetPlayer) (delegate Custom|Player_interact_Button)))))

(event Collision|EventActorBeginOverlap
  (params (OtherActor :type Actor%20Object%20Reference)))

(event EventTick
  (params (DeltaSeconds :type Float%20%28single-precision%29)))

(fn ConstructionScript)