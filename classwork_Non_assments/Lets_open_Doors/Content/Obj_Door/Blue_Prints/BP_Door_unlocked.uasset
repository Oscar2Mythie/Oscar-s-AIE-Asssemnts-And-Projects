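; BP_Door_unlocked is a sensor-driven door that opens and closes automatically for an actor with a matching name.
; Door_Sensor overlap events compare the other actor's display name against PassName, printing debug strings along the way.
; On a match, entering eases DoorAnchor to an offset relative location over a timed move, and leaving eases it back to the relative origin.
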(event OnComponentBeginOverlap(Door_Sensor)
  (params (OverlappedComponent :type Primitive%20Component%20Object%20Reference) (OtherActor :type Actor%20Object%20Reference) (OtherComp :type Primitive%20Component%20Object%20Reference) (OtherBodyIndex :type Integer) (bFromSweep :type Boolean) (SweepResult :type Hit%20Result%20Structure%20%28by%20ref%29))
  ;[0.3798 0.6987 1 1 36] Basic Enter and exit opening door
  (Development|PrintString "Hello")
  (if (Utilities|Enum|Equal(Enum) (Utilities|GetDisplayName OtherActor) (Variables|Default|GetPass_Name))
    (Development|PrintString "Player!")
    (Components|MoveComponentTo (Variables|Default|GetDoor%20Anchor) "0.000000,-50.000000,-110.000000" "0, 0, 0" true true 2.0 false)))

(event OnComponentEndOverlap(Door_Sensor)
  (params (OverlappedComponent :type Primitive%20Component%20Object%20Reference) (OtherActor :type Actor%20Object%20Reference) (OtherComp :type Primitive%20Component%20Object%20Reference) (OtherBodyIndex :type Integer))
  ;[0.3798 0.6987 1 1 36] Basic Enter and exit opening door
  (Development|PrintString "Hello")
  (if (Utilities|Enum|Equal(Enum) (Utilities|GetDisplayName OtherActor) (Variables|Default|GetPass_Name))
    (Development|PrintString "Player")
    (Components|MoveComponentTo (Variables|Default|GetDoor%20Anchor) "0, 0, 0" "0, 0, 0" true true 2.0 false)))

(event EventBeginPlay)

(event EventTick
  (params (DeltaSeconds :type Float%20%28single-precision%29)))

(fn ConstructionScript)