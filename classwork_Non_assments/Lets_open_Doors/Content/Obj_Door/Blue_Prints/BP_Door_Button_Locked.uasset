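; Locked golden door that splits into four panels and opens when its button is pressed.
; The Open_button_locked_Door event uses a Sequence to start all four panel animations together.
; Each panel runs chained, eased MoveComponentTo calls: move to an offset, rotate 45 degrees, then slide diagonally outward.
; The file contains no close, lock-check or button-detection logic.
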(event Custom|Open_button_locked_Door
  ;[0.3798 0.6987 1 1 36] Open the Golden Door when button is pressed
  (Utilities|FlowControl|Sequence
    (:then_0
      (Components|MoveComponentTo (Variables|Default|GetTLhs_Door) "-37.500000,0.000000,75.000000" "0, 0, 0" false true 1.0 false)
      (Components|MoveComponentTo (Variables|Default|GetTLhs_Door) "-37.500000,0.000000,75.000000" "-45.000000,0.000000,0.000000" true true 1.0 false)
      (Components|MoveComponentTo (Variables|Default|GetTLhs_Door) "-52.500000,0.000000,90.000000" "-45.000000,0.000000,0.000000" false true 1.0 false))
    (:then_1
      (Components|MoveComponentTo (Variables|Default|GetBLhs_Door) "-37.500000,0.000000,25.000000" "0, 0, 0" false true 1.0 false)
      (Components|MoveComponentTo (Variables|Default|GetBLhs_Door) "-37.500000,0.000000,25.000000" "45.000000,0.000000,0.000000" true true 1.0 false)
      (Components|MoveComponentTo (Variables|Default|GetBLhs_Door) "-58.000000,0.000000,-10.000000" "45.000000,0.000000,0.000000" false true 1.0 false))
    (:then_2
      (Components|MoveComponentTo (Variables|Default|GetTRhs_Door) "37.500000,0.000000,75.000000" "0, 0, 0" false true 1.0 false)
      (Components|MoveComponentTo (Variables|Default|GetTRhs_Door) "37.500000,0.000000,75.000000" "45.000000,0.000000,0.000000" true true 1.0 false)
      (Components|MoveComponentTo (Variables|Default|GetTRhs_Door) "52.500000,0.000000,90.000000" "45.000000,0.000000,0.000000" false true 1.0 false))
    (:then_3
      (Components|MoveComponentTo (Variables|Default|GetBRhs_Door) "37.500000,0.000000,25.000000" "0, 0, 0" false true 1.0 false)
      (Components|MoveComponentTo (Variables|Default|GetBRhs_Door) "37.500000,0.000000,25.000000" "-45.000000,0.000000,0.000000" true true 1.0 false)
      (Components|MoveComponentTo (Variables|Default|GetBRhs_Door) "58.000000,0.000000,-10.000000" "-45.000000,0.000000,0.000000" false true 1.0 false))))

(event EventBeginPlay)

(event EventTick
  (params (DeltaSeconds :type Float%20%28single-precision%29)))

(fn ConstructionScript)