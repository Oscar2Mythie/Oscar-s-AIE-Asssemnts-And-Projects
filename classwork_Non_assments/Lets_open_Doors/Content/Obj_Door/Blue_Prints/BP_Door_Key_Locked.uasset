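; BP_Door_Key_Locked is a key-locked door that rotates open and closed as a matching actor enters and leaves its sensor.
; Key_Unlock_Door sets KeyFound, which gates both overlap handlers along with a display-name check against PassName.
; MoveComponentTo eases the door and anchor between poses.
; The first opening increments DoorsOpen on the GM_Gamplay actor, found at BeginPlay through GetAllActorsOfClass.
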(event OnComponentBeginOverlap(Door_Sensor)
  (params (OverlappedComponent :type Primitive%20Component%20Object%20Reference) (OtherActor :type Actor%20Object%20Reference) (OtherComp :type Primitive%20Component%20Object%20Reference) (OtherBodyIndex :type Integer) (bFromSweep :type Boolean) (SweepResult :type Hit%20Result%20Structure%20%28by%20ref%29))
  (bind _gm_gameplay (Variables|Default|GetGM_Gameplay))
  ;[0.3798 0.6987 1 1 36] Basic Enter and exit opening door
  (Development|PrintString "Hello")
  (if (Utilities|Enum|Equal(Enum) (Utilities|GetDisplayName OtherActor) (Variables|Default|GetPass_Name))
    (if (Variables|Default|GetKey_Found)
      (Utilities|FlowControl|Sequence
        (:then_0
          (Development|PrintString "Player!")
          (Components|MoveComponentTo (Variables|Default|GetThe_Door) "0.000000,0.000000,-550.000000" "0.000000,90.000000,0.000000" true true 2.0 false)
          (Components|MoveComponentTo (Variables|Default|GetDoor%20Anchor) "-12.500000,0.000000,100.000000" "0.000000,90.000000,0.000000" true true 2.0 false))
        (:then_1
          (if (Variables|Default|Getfirst%20time%20opened)
            (bind _output_get (Variables|/Game/Game_Modes/GM_Gamplay.GM_Gamplay_C|SetDoors_Open _gm_gameplay (+ 1 (Variables|/Game/Game_Modes/GM_Gamplay.GM_Gamplay_C|GetDoors_Open _gm_gameplay))))
            (Variables|Default|Setfirst%20time%20opened false)
            (Development|PrintString (Utilities|String|ToString(Integer) _output_get))))))))

(event OnComponentEndOverlap(Door_Sensor)
  (params (OverlappedComponent :type Primitive%20Component%20Object%20Reference) (OtherActor :type Actor%20Object%20Reference) (OtherComp :type Primitive%20Component%20Object%20Reference) (OtherBodyIndex :type Integer))
  ;[0.3798 0.6987 1 1 36] Basic Enter and exit opening door
  (Development|PrintString "Hello")
  (if (Utilities|Enum|Equal(Enum) (Utilities|GetDisplayName OtherActor) (Variables|Default|GetPass_Name))
    (if (Variables|Default|GetKey_Found)
      (Development|PrintString "Player")
      (Components|MoveComponentTo (Variables|Default|GetDoor%20Anchor) "-12.500000,0.000000,100.000000" "0, 0, 0" true true 2.0 false)
      (Components|MoveComponentTo (Variables|Default|GetThe_Door) "0.000000,0.000000,-550.000000" "0, 0, 0" true true 2.0 false))))

(event Custom|Key_Unlock_Door
  ;[0.3798 0.6987 1 1 36] Basic Enter and exit opening door
  (Variables|Default|SetKey_Found true))

(event EventBeginPlay
  (bind _outactors (Actor|GetAllActorsOfClass "/Game/Game_Modes/GM_Gamplay.GM_Gamplay_C"))
  (Variables|Default|SetGM_Gameplay (Utilities|Array|Get(acopy) _outactors)))

(event EventTick
  (params (DeltaSeconds :type Float%20%28single-precision%29)))

(fn ConstructionScript)