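; BP_Door_End is an end door that activates once the door count in GM_Gamplay matches its required number.
; BeginPlay caches GM_Gamplay via GetAllActorsOfClass, and Tick spins the BallAnhcor component while the counts match, at a frame-rate-dependent speed.
; Box overlap prints a debug message, then moves BallAnhcor to a raised relative position if the count matches and the actor's display name equals PassName.
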(event OnComponentBeginOverlap(Box)
  (params (OverlappedComponent :type Primitive%20Component%20Object%20Reference) (OtherActor :type Actor%20Object%20Reference) (OtherComp :type Primitive%20Component%20Object%20Reference) (OtherBodyIndex :type Integer) (bFromSweep :type Boolean) (SweepResult :type Hit%20Result%20Structure%20%28by%20ref%29))
  (Development|PrintString "Hello")
  (if (and (== (Variables|/Game/Game_Modes/GM_Gamplay.GM_Gamplay_C|GetDoors_Open (Variables|Default|GetGM_Gameplay)) (Variables|Default|GetNeeded_Doors_Open)) (Utilities|Enum|Equal(Enum) (Utilities|GetDisplayName OtherActor) (Variables|Default|GetPass_Name)))
    (Components|MoveComponentTo (Variables|Default|GetBall%20anhcor) "0.000000,0.000000,100.000000" "0, 0, 0" false false 1.0 false)))

(event EventBeginPlay
  (bind _outactors (Actor|GetAllActorsOfClass "/Game/Game_Modes/GM_Gamplay.GM_Gamplay_C"))
  (Variables|Default|SetGM_Gameplay (Utilities|Array|Get(acopy) _outactors)))

(event Collision|EventActorBeginOverlap
  (params (OtherActor :type Actor%20Object%20Reference)))

(event EventTick
  (params (DeltaSeconds :type Float%20%28single-precision%29))
  (if (== (Variables|/Game/Game_Modes/GM_Gamplay.GM_Gamplay_C|GetDoors_Open (Variables|Default|GetGM_Gameplay)) (Variables|Default|GetNeeded_Doors_Open))
    (Transformation|AddLocalRotation (Variables|Default|GetBall%20anhcor) "0.000000,5.000000,0.000000" false false)))

(fn ConstructionScript)